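; Test Blueprint that lets gamepad shoulder buttons toggle boosted walk speed and jump velocity on the third-person character.
; BeginPlay finds the character and caches its default MaxWalkSpeed and JumpZVelocity.
; While a toggle is on, Tick reapplies the new value every frame; toggling off restores the cached default and prints the state.
; Unconnected leftover nodes for camera boom and rotation settings never execute.
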(event EventBeginPlay
  ;[1 0 0 0.5] Replace Reference with Player
  (bind _returnvalue (Actor|GetActorOfClass "/Game/ThirdPerson/Blueprints/BP_ThirdPersonCharacter.BP_ThirdPersonCharacter_C"))
  ;[0.15 0.09528 0.05146 0.5] Get Default Values
  (Variables|Default|SetspeedInitial (Variables|/Script/Engine.CharacterMovementComponent|GetMaxWalkSpeed (Variables|/Script/Engine.Character|GetCharacterMovement _returnvalue)))
  (Variables|Default|SetjumpInitial (Variables|/Script/Engine.CharacterMovementComponent|GetJumpZVelocity (Variables|/Script/Engine.Character|GetCharacterMovement _returnvalue)))
  (Variables|Default|SetdefaultValuesGotten true)
  (if (Variables|Default|GetspeedUp)
    (Development|PrintString "Speed Up Activated"))
  (if (Variables|Default|GetjumpUp)
    (Development|PrintString "Jump Up Activated")))

(event Collision|EventActorBeginOverlap
  (params (OtherActor :type Actor%20Object%20Reference)))

(event EventTick
  (params (DeltaSeconds :type Float%20%28single-precision%29))
  (if (Variables|Default|GetdefaultValuesGotten)
    (Utilities|FlowControl|Sequence
      (:then_0
        ;[0.15 0.15 0.313 0.5] Modify Max Walk Speed
        (if (Variables|Default|GetspeedUp)
          ;;[1 0 0 0.5 13] Replace Reference with Max Walk Speed
          (Variables|/Script/Engine.CharacterMovementComponent|SetMaxWalkSpeed (Variables|/Script/Engine.Character|GetCharacterMovement (stale EventBeginPlay _returnvalue)) (Variables|Default|GetspeedNew))))
      (:then_1
        ;[0.227 0.2016 0.15 0.502] Modify Jump Z Velocity
        (if (Variables|Default|GetjumpUp)
          ;;[1 0 0 0.5 13] Replace Reference with Jump Z Velocity
          (Variables|/Script/Engine.CharacterMovementComponent|SetJumpZVelocity (Variables|/Script/Engine.Character|GetCharacterMovement (stale EventBeginPlay _returnvalue)) (Variables|Default|GetjumpNew)))))))

(event Input|GamepadEvents|GamepadRightShoulder
  (params (Key :type Key%20Structure :default "None"))
  ;[0.15 0.2957 0.15 0.5] Jump Z Velocity Modifier
  (:Pressed
    (if (Variables|Default|GetjumpUp)
      (Variables|Default|SetjumpUp false)
      (Development|PrintString "Jump Up Deactivated" true false)
      ;[0.01963 0.15 0.1435 0.5 17] Values Reset Here in Case They Are Already Modified in Runtime; Avoids Locking Speed/Jump Height in That Case
      (Variables|/Script/Engine.CharacterMovementComponent|SetJumpZVelocity (Variables|/Script/Engine.Character|GetCharacterMovement (stale EventBeginPlay _returnvalue)) (Variables|Default|GetjumpInitial))
      (else
        (Variables|Default|SetjumpUp true)
        (Development|PrintString "Jump Up Activated" true false)))))

(event Input|GamepadEvents|GamepadLeftShoulder
  (params (Key :type Key%20Structure :default "None"))
  ;[0.2957 0.15 0.226 0.5] Max Walk Speed Modifier
  (:Pressed
    (if (Variables|Default|GetspeedUp)
      (Variables|Default|SetspeedUp false)
      (Development|PrintString "Speed Up Deactivated" true false)
      ;[0.01963 0.15 0.1435 0.5 17] Values Reset Here in Case They Are Already Modified in Runtime; Avoids Locking Speed/Jump Height in That Case
      (Variables|/Script/Engine.CharacterMovementComponent|SetMaxWalkSpeed (Variables|/Script/Engine.Character|GetCharacterMovement (stale EventBeginPlay _returnvalue)) (Variables|Default|GetspeedInitial))
      (else
        (Variables|Default|SetspeedUp true)
        (Development|PrintString "Speed Up Activated" true false)))))

(fn ConstructionScript)