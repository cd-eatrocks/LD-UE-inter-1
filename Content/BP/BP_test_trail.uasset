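; BP_test_trail is a test actor that leaves a short-lived trail at the third-person character's position.
; Each Tick it looks up the character and, if CreateMesh is set, uses a Delay to space out BP_trailMesh spawns at that location, each expiring after TrailLifeSpan.
; If CreatePoints is set, it also draws three colored debug points every Tick below, at and above the character's location, with the same lifespan.
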(event EventBeginPlay)

(event Collision|EventActorBeginOverlap
  (params (OtherActor :type Actor%20Object%20Reference)))

(event EventTick
  (params (DeltaSeconds :type Float%20%28single-precision%29))
  (bind _returnvalue (Actor|GetActorOfClass "/Game/ThirdPerson/Blueprints/BP_ThirdPersonCharacter.BP_ThirdPersonCharacter_C"))
  (Utilities|FlowControl|Sequence
    (:then_0
      (if (Variables|Default|GetcreateMesh)
        (Utilities|FlowControl|Delay (Variables|Default|GetmeshSpawnDelay))
        (bind _returnvalue_2 (Game|SpawnActorfromClass "/Game/BP/BP_trailMesh.BP_trailMesh_C" (Math|Conversions|ToTransform(Vector) (Math|Vector|MakeVector (.x (Transformation|GetActorLocation _returnvalue)) (.y (Transformation|GetActorLocation _returnvalue)) (.z (Transformation|GetActorLocation _returnvalue)))) "Undefined" "MultiplyWithRoot" 0 0))
        (Actor|SetLifeSpan _returnvalue_2 (Variables|Default|GettrailLifeSpan))))
    (:then_1
      (if (Variables|Default|GetcreatePoints)
        (Utilities|FlowControl|Sequence
          (:then_0
            (Rendering|Debug|DrawDebugPoint (Math|Vector|MakeVector (.x (Transformation|GetActorLocation _returnvalue)) (.y (Transformation|GetActorLocation _returnvalue)) (- (.z (Transformation|GetActorLocation _returnvalue)) 8e+01)) 5.0 "(R=0.000000,G=0.194890,B=0.635417,A=1.000000)" (Variables|Default|GettrailLifeSpan)))
          (:then_1
            (Rendering|Debug|DrawDebugPoint (Math|Vector|MakeVector (.x (Transformation|GetActorLocation _returnvalue)) (.y (Transformation|GetActorLocation _returnvalue)) (.z (Transformation|GetActorLocation _returnvalue))) 5.0 "(R=0.214796,G=0.635417,B=0.062316,A=1.000000)" (Variables|Default|GettrailLifeSpan)))
          (:then_2
            (Rendering|Debug|DrawDebugPoint (Math|Vector|MakeVector (.x (Transformation|GetActorLocation _returnvalue)) (.y (Transformation|GetActorLocation _returnvalue)) (+ (.z (Transformation|GetActorLocation _returnvalue)) 8e+01)) 5.0 "(R=0.635417,G=0.379715,B=0.044291,A=1.000000)" (Variables|Default|GettrailLifeSpan))))))))

(fn ConstructionScript)